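; Tactical camera pawn that pans, zooms and rotates from player input.
; Axis input shifts a desired location along the actor's forward and right vectors, and the actor interpolates toward it at CameraSpeed.
; Rotation presses offset a desired rotation in 45-degree increments, while zoom presses adjust spring arm length by its initial value, clamped to limits.
; Rotation and zoom apply only one interpolation step per press, with no Tick follow-through.
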(event `self.ReceiveBeginPlay`
  (set `self.LocationDesired` (`self.K2_GetActorLocation`))
  (set `self.ZoomDesired` (`SpringArmComponent.TargetArmLength` (`self.SpringArm`)))
  (set `self.RotationDesired` (`self.K2_GetActorRotation`)))

(event `InputAxis|InputAxis_Forward`
  (params (AxisValue :type "Float (single-precision)"))
  (bind _output_get (set `self.LocationDesired` (+ (`self.LocationDesired`) (* (`self.GetActorForwardVector`) (* AxisValue 40.0)))))
  (`self.K2_SetActorLocation` (`KismetMathLibrary.VInterpTo` (`self.K2_GetActorLocation`) _output_get (`GameplayStatics.GetWorldDeltaSeconds`) (`self.CameraSpeed`))))

(event `InputAxis|InputAxis_Right`
  (params (AxisValue :type "Float (single-precision)"))
  (bind _output_get (set `self.LocationDesired` (+ (`self.LocationDesired`) (* (`self.GetActorRightVector`) (* AxisValue 40.0)))))
  (`self.K2_SetActorLocation` (`KismetMathLibrary.VInterpTo` (`self.K2_GetActorLocation`) _output_get (`GameplayStatics.GetWorldDeltaSeconds`) (`self.CameraSpeed`))))

(event `InputAction|Zoom Camera In`
  (params (Key :type "Key Structure"))
  (bind _springarm (`self.SpringArm`))
  (bind _targetarmlength (`SpringArmComponent.TargetArmLength` _springarm))
  (:`Pressed`
    (set `SpringArmComponent.TargetArmLength` (`KismetMathLibrary.FClamp` (`KismetMathLibrary.FInterpTo` _targetarmlength (+ _targetarmlength (`self.ZoomDesired`)) (`GameplayStatics.GetWorldDeltaSeconds`) (`self.CameraSpeed`)) (`self.MinArmLength`) (`self.MaxArmLength`)) _springarm)))

(event `InputAction|Zoom Camera Out`
  (params (Key :type "Key Structure"))
  (bind _springarm (`self.SpringArm`))
  (bind _targetarmlength (`SpringArmComponent.TargetArmLength` _springarm))
  (:`Pressed`
    (set `SpringArmComponent.TargetArmLength` (`KismetMathLibrary.FClamp` (`KismetMathLibrary.FInterpTo` _targetarmlength (- _targetarmlength (`self.ZoomDesired`)) (`GameplayStatics.GetWorldDeltaSeconds`) (`self.CameraSpeed`)) (`self.MinArmLength`) (`self.MaxArmLength`)) _springarm)))

(event `InputAction|InputAction_RightRotation`
  (params (Key :type "Key Structure"))
  (:`Pressed`
    (bind _output_get (set `self.RotationDesired` (`KismetMathLibrary.ComposeRotators` (`self.RotationDesired`) (struct :`Yaw` -45.0))))
    (`self.K2_SetActorRotation` (`KismetMathLibrary.RInterpTo` (`self.K2_GetActorRotation`) _output_get (`GameplayStatics.GetWorldDeltaSeconds`) (`self.CameraSpeed`)))))

(event `InputAction|InputAction_LeftRotation`
  (params (Key :type "Key Structure"))
  (:`Pressed`
    (bind _output_get (set `self.RotationDesired` (`KismetMathLibrary.ComposeRotators` (`self.RotationDesired`) (struct :`Yaw` 45.0))))
    (`self.K2_SetActorRotation` (`KismetMathLibrary.RInterpTo` (`self.K2_GetActorRotation`) _output_get (`GameplayStatics.GetWorldDeltaSeconds`) (`self.CameraSpeed`)))))

(fn `UserConstructionScript`)